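; BP_NightSkyGameInstance is the NightSkyEngine game instance Blueprint that handles online session events and replay search results.
; When the instance is the host, HostSession sets up an Advanced Session tagged with the game name.
; Accepted session invites join the invited session directly.
; Completed replay searches are forwarded to the first replay menu widget found, provided the player controller is the menu controller.
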(event `HostSession`
  (if (`self.IsHost`)
    (`CreateSessionCallbackProxyAdvanced.CreateAdvancedSession` (`|MakeArray` (`AdvancedSessionsLibrary.MakeLiteralSessionPropertyString` "GameName" "NightSkyEngine")) (`GameplayStatics.GetPlayerController` 0) 4)))

(event `self.BP_OnFindReplaysComplete`
  (params (AllReplays :type "Array of ReplaySaveInfo Object Reference (by ref)"))
  (cast `/Game/Blueprints/Menu/BP_MenuPlayerController` (`GameplayStatics.GetPlayerController` 0))
  (bind _foundwidgets (`WidgetBlueprintLibrary.GetAllWidgetsOfClass` "/Game/UI/Replay/WBP_ReplayMenu.WBP_ReplayMenu_C" false))
  (`/Game/UI/Replay/WBP_ReplayMenu.OnFindReplays` (`|GetArrayItem` _foundwidgets) AllReplays))

(event `self.OnSessionInviteAccepted`
  (params (LocalPlayerNum :type Integer) (PersonInvited :type "BPUniqueNetId Structure") (SessionToJoin :type "BlueprintSessionResult Structure (by ref)"))
  (`JoinSessionCallbackProxy.JoinSession` (`GameplayStatics.GetPlayerController` 0) SessionToJoin))