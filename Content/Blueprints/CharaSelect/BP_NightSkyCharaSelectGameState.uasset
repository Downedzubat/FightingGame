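; Game state for the character select screen, resetting match picks and providing loaded character and stage data.
; On BeginPlay it clears the game instance's BattleData player list and color indices, then resizes both to six slots.
; Separate gather functions enumerate primary asset IDs, load each synchronously, and append the results to the CharaDatas and StageDatas arrays.
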(event `self.ReceiveBeginPlay`
  (bind _asbp_night_sky_game_instance (cast `/Game/Blueprints/Common/BP_NightSkyGameInstance` (`GameplayStatics.GetGameInstance`)))
  (bind (_playerlist _colorindices) (break `BattleData` (`NightSkyGameInstance.BattleData` _asbp_night_sky_game_instance)))
  (`KismetArrayLibrary.Array_Clear` _playerlist)
  (`KismetArrayLibrary.Array_Resize` _playerlist 6)
  (`KismetArrayLibrary.Array_Clear` _colorindices)
  (`KismetArrayLibrary.Array_Resize` _colorindices 6))

(fn `GatherCharaData`
  (bind _outprimaryassetidlist (`KismetSystemLibrary.GetPrimaryAssetIdList` "PrimaryCharaData"))
  (for _array_element _outprimaryassetidlist
    (bind _returnvalue (`KismetSystemLibrary.LoadAsset_Blocking` (`KismetSystemLibrary.GetSoftObjectReferenceFromPrimaryAssetId` _array_element)))
    (bind _asprimary_chara_data (cast `PrimaryCharaData` _returnvalue))
    (`KismetArrayLibrary.Array_Add` (`self.CharaDatas`) _asprimary_chara_data)))

(fn `GatherStageData`
  (bind _outprimaryassetidlist (`KismetSystemLibrary.GetPrimaryAssetIdList` "PrimaryStageData"))
  (for _array_element _outprimaryassetidlist
    (bind _returnvalue (`KismetSystemLibrary.LoadAsset_Blocking` (`KismetSystemLibrary.GetSoftObjectReferenceFromPrimaryAssetId` _array_element)))
    (bind _asprimary_stage_data (cast `PrimaryStageData` _returnvalue))
    (`KismetArrayLibrary.Array_Add` (`self.StageDatas`) _asprimary_stage_data)))

(fn `UserConstructionScript`)